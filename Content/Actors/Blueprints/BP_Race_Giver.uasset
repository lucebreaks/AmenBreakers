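; Race-giver actor that starts a checkpoint race against an AI adversary when its dialog finishes with Started set.
; It spawns checkpoints at six placed points, registers them with BP_RaceTracker and teleports the player to the start.
; It then spawns the adversary, shows the race HUD, disables input and calls RaceSetup.
; Resettable DoOnce gates guard both stages, and Tick re-invokes DialogFinished while the tracker reports RaceOver.
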(event Custom|ResetRace
  (bind _returnvalue (Game|GetPlayerController 0))
  (Utilities|FlowControl|DoOnce false) ; enters at Reset
)

(event EventBeginPlay
  (|CallParentFunction)
  (bind _returnvalue (Actor|GetActorOfClass "/Game/Actors/Blueprints/Race_Items/BP_RaceTracker.BP_RaceTracker_C"))
  (Variables|Default|SetRace_tracker_ref _returnvalue))

(event Collision|EventActorBeginOverlap
  (params (OtherActor :type Actor%20Object%20Reference)))

(event EventOnReset
  (bind _returnvalue (Game|GetPlayerController 0))
  (bind _player_spawn_point (Variables|Default|GetPlayer_Spawn_Point))
  (bind _returnvalue_2 (Transformation|GetWorldTransform _player_spawn_point))
  (Utilities|FlowControl|DoOnce false) ; enters at Reset
)

(event EventDialogFinished
  (bind _returnvalue (Game|GetPlayerController 0))
  (bind _player_spawn_point (Variables|Default|GetPlayer_Spawn_Point))
  (bind _returnvalue_2 (Transformation|GetWorldTransform _player_spawn_point))
  (if (Variables|Default|GetStarted?)
    (Utilities|FlowControl|DoOnce false
      (:Completed
        (for _array_element (Utilities|Array|MakeArray (Variables|Default|GetCheckpoint1) (Variables|Default|GetCheckpoint2) (Variables|Default|GetCheckpoint3) (Variables|Default|GetCheckpoint4) (Variables|Default|GetCheckpoint5) (Variables|Default|GetCheckpoint6))
          (bind _returnvalue_3 (Game|SpawnActorfromClass "/Game/Actors/Blueprints/Race_Items/BP_Checkpoint.BP_Checkpoint_C" (Transformation|GetWorldTransform _array_element) "Undefined" 0 0))
          (Utilities|Array|Add (Variables|/Game/Actors/Blueprints/Race_Items/BP_RaceTracker.BP_RaceTracker_C|GetCheckpoints (Variables|Default|GetRace_tracker_ref)) _returnvalue_3))
        (Transformation|Teleport (Game|GetPlayerCharacter 0) (.location _returnvalue_2) (.rotation _returnvalue_2))
        (Utilities|FlowControl|DoOnce false
          (:Completed
            (Game|SpawnActorfromClass "/Game/Actors/Blueprints/BP_AI_Adversary.BP_AI_Adversary_C" (Transformation|GetWorldTransform (Variables|Default|GetAI_Spawn_Point)) "Undefined" 0 0)
            (bind _returnvalue_4 (UserInterface|CreateWidget "/Game/HUD/WBP_Race_HUD.WBP_Race_HUD_C" _returnvalue))
            (Variables|Default|SetRace_hud_ref _returnvalue_4)
            (UserInterface|Viewport|AddtoViewport _returnvalue_4 0)
            (Input|DisableInput (Game|GetPlayerCharacter 0) _returnvalue)
            (Default|RaceSetup (Variables|Default|GetRace_tracker_ref))))))))

(event EventTick
  (params (DeltaSeconds :type Float%20%28single-precision%29))
  (if (Variables|/Game/Actors/Blueprints/Race_Items/BP_RaceTracker.BP_RaceTracker_C|GetRaceOver (Variables|Default|GetRace_tracker_ref))
    (CallFunction|DialogFinished)))

(fn ConstructionScript
  (|CallParentFunction))