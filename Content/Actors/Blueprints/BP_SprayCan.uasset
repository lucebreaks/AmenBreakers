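; BP_SprayCan is a pickup that refills the player character's spray count.
; Overlapping its Sphere with a BP_PlayerCharacter tagged PlayerChar adds CanAmount to SprayCount.
; The existing count is clamped to 0–30 before the addition, so the result can exceed that cap.
; After pickup the actor hides and disables collision, then reappears and re-enables collision following a 45-second delay.
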(event OnComponentBeginOverlap(Sphere)
  (params (OverlappedComponent :type Primitive%20Component%20Object%20Reference) (OtherActor :type Actor%20Object%20Reference) (OtherComp :type Primitive%20Component%20Object%20Reference) (OtherBodyIndex :type Integer) (bFromSweep :type Boolean) (SweepResult :type Hit%20Result%20Structure%20%28by%20ref%29))
  (Utilities|IsValid OtherActor
    (:Is%20Valid
      (if (Actor|ActorHasTag OtherActor "PlayerChar")
        (bind _asbp_player_character (Utilities|Casting|CastToBP_PlayerCharacter OtherActor))
        (Variables|/Game/Actors/Blueprints/BP_PlayerCharacter.BP_PlayerCharacter_C|SetSprayCount _asbp_player_character (+ (Math|Integer|Clamp(Integer) (Variables|/Game/Actors/Blueprints/BP_PlayerCharacter.BP_PlayerCharacter_C|GetSprayCount _asbp_player_character) 0 30) (Variables|Default|GetCanAmount)))
        (Rendering|SetActorHiddenInGame true)
        (Collision|SetActorEnableCollision false)
        (Utilities|FlowControl|Delay 45.0)
        (Rendering|SetActorHiddenInGame false)
        (Collision|SetActorEnableCollision true)))))

(event EventBeginPlay)

(event Collision|EventActorBeginOverlap
  (params (OtherActor :type Actor%20Object%20Reference)))

(event EventTick
  (params (DeltaSeconds :type Float%20%28single-precision%29)))

(fn ConstructionScript)