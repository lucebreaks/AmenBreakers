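; BP_RaceTracker is an actor that runs a checkpoint race, tracking progress through an ordered checkpoint array over multiple laps.
; It binds each checkpoint's clear callback and activates one checkpoint at a time, wrapping to the first on each new lap.
; After the final lap, it resets race state, destroys BP_AI_Adversary, then hides BP_Race_Giver's HUD and marks it finished.
; AIWins does not change the outcome, and LapCheck is empty.
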(event Custom|Checkpoint%20Cleared
  (bind _checkpoints (Variables|Default|GetCheckpoints))
  (bind _output_get (Variables|Default|SetCheckpointNumber (+ (Variables|Default|GetCheckpointNumber) 1)))
  (if (>= (Variables|Default|GetCheckpointNumber) (Utilities|Array|Length (Variables|Default|GetCheckpoints)))
    (Variables|Default|SetCurrentLap (+ (Variables|Default|GetCurrentLap) 1))
    (Variables|Default|SetCheckpointNumber 0)
    (if (>= (Variables|Default|GetCurrentLap) (Variables|Default|GetMax_Laps))
      (CallFunction|RaceFinishCheck)
      (else
        (Default|ActivateCheckPoint (Utilities|Array|Get(acopy) _checkpoints))))
    (else
      (Default|ActivateCheckPoint (Utilities|Array|Get(acopy) _checkpoints _output_get)))))

(event Custom|StartRaceSequence
  (bind _checkpoints (Variables|Default|GetCheckpoints))
  (CallFunction|RaceStart)
  (for _array_element _checkpoints
    (EventDispatchers|AssignCheckpointClear _array_element (delegate Custom|Checkpoint%20Cleared))
    ;[1 1 1] Setup first Checkpoint
    (Default|DeactivateCheckpoint _array_element))
  (Default|ActivateCheckPoint (Utilities|Array|Get(acopy) _checkpoints)))

(fn ConstructionScript)

(fn RaceFinishCheck
  (if (Variables|Default|GetAI_Wins)
    (Variables|Default|SetRaceOver true)
    (else
      (Variables|Default|SetRaceOver true)))
  (CallFunction|StopandResetRace)
  (bind _returnvalue (Actor|GetActorOfClass "/Game/Actors/Blueprints/BP_Race_Giver.BP_Race_Giver_C"))
  (Widget|SetVisibility (Variables|/Game/Actors/Blueprints/BP_Race_Giver.BP_Race_Giver_C|GetRace_hud_ref _returnvalue) "Hidden")
  (Variables|/Game/Actors/Blueprints/QuestGiver_BP.QuestGiver_BP_C|SetFinished? _returnvalue true))

(fn LapCheck)

(fn RaceSetup
  (for (_array_element _array_index) (Variables|Default|GetCheckpoints)
    (Variables|/Game/Actors/Blueprints/Race_Items/BP_Checkpoint.BP_Checkpoint_C|SetCheckpoint_Number _array_element _array_index)
    (Default|DeactivateCheckpoint _array_element)))

(fn RaceStart
  (Default|ActivateCheckPoint (Utilities|Array|Get(acopy) (Variables|Default|GetCheckpoints))))

(fn StopandResetRace
  (for _array_element (Variables|Default|GetCheckpoints)
    (Default|DeactivateCheckpoint _array_element))
  (Variables|Default|SetAI_Wins false)
  (Variables|Default|SetRaceStart? false)
  (Variables|Default|SetCurrentLap 0)
  (bind _returnvalue (Actor|GetActorOfClass "/Game/Actors/Blueprints/BP_AI_Adversary.BP_AI_Adversary_C"))
  (Actor|DestroyActor _returnvalue))