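; QuestSpray is a quest giver whose territorial tagger dialog challenges the player to cover a tag high on a billboard.
; On BeginPlay it sets start, mid and end dialog lines after the parent's setup, then spawns a TrickSpray at SprayPos, rotated to lie on the wall.
; When dialog finishes and the quest is not yet Finished, it unhides the spray's Helper component to open up the spot.
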(event EventBeginPlay
  (bind _spray_pos (Variables|Default|GetSpray%20pos))
  (bind _returnvalue (Transformation|GetWorldTransform _spray_pos))
  (bind (_location _rotation _scale) (Math|Transform|BreakTransform _returnvalue))
  (bind (_roll _pitch _yaw) (Math|Rotator|BreakRotator _rotation))
  (|CallParentFunction)
  ;[1 1 1] Set Up Dialog
  (Variables|Default|SetStartDialog "Whatchu' doing up here on the hill? The hill is my territory. See that tag in the middle of the billboard? That's mine. That's how you know I own this zone.")
  (Variables|Default|SetMidDialog "Unless you think you can cover my tag way up there, get lost!")
  (Variables|Default|SetEndDialog "What the f- How did you cover my tag? Now all the homies are gonna call me lame...")
  ;[1 1 1] spawn quest spray and rotate it to wall
  (bind _returnvalue_2 (Game|SpawnActorfromClass "/Game/TrickSpray.TrickSpray_C" (Math|Transform|MakeTransform _location (Math|Rotator|MakeRotator (+ _roll 9e+01) _pitch (+ _yaw -9e+01)) _scale) "Undefined" 0 0))
  (Variables|Default|SetTrickSpray _returnvalue_2))

(event EventDialogFinished
  ;[1 1 1] Make the Spot sprayable after talking to the quest giver
  (if (not (Variables|Default|GetFinished?))
    (Development|SetHiddeninGame (Variables|/Game/SprayDecals/Spray_Blueprint.Spray_Blueprint_C|GetHelper (Variables|Default|GetTrickSpray)) false false)))

(fn ConstructionScript
  (|CallParentFunction))