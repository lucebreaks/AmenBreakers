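; QuestGiver_BP is a quest-giver actor that shows dialogue matching the state of its quest.
; BeginPlay creates a hidden DialogWidget, then calls Ready, an empty event like DialogFinished.
; DialogPopup shows the widget with start, middle or end text based on Started and Finished, setting Started on first use and hiding Notification once finished.
; The player leaving TalkZone hides visible dialogue and calls DialogFinished.
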(event OnComponentEndOverlap(TalkZone)
  (params (OverlappedComponent :type Primitive%20Component%20Object%20Reference) (OtherActor :type Actor%20Object%20Reference) (OtherComp :type Primitive%20Component%20Object%20Reference) (OtherBodyIndex :type Integer))
  (bind _dialogwidget (Variables|Default|GetDialogWidget))
  ;[1 1 1] Hide text when player walks away
  (if (Widget|IsVisible _dialogwidget)
    (Utilities|Casting|CastToBP_PlayerCharacter OtherActor)
    (Widget|SetVisibility _dialogwidget "Hidden")
    (CallFunction|DialogFinished)))

(event Custom|DialogFinished)

(event Custom|Ready)

(event EventBeginPlay
  ;[1 1 1] Create Dialog interaction, hidden
  (bind _returnvalue (UserInterface|CreateWidget "/Game/HUD/DialogWidget.DialogWidget_C"))
  (Widget|SetVisibility _returnvalue "Hidden")
  (bind _output_get (Variables|Default|SetDialogWidget _returnvalue))
  (UserInterface|Viewport|AddtoViewport _output_get 0)
  (CallFunction|Ready))

(fn ConstructionScript)

(fn DialogPopup
  (bind _dialogwidget (Variables|Default|GetDialogWidget))
  ;[1 1 1] Make dialog visible and set text depending on state
  (Widget|SetVisibility _dialogwidget "Visible")
  (if (Variables|Default|GetStarted?)
    (if (Variables|Default|GetFinished?)
      (Variables|/Game/HUD/DialogWidget.DialogWidget_C|SetLine _dialogwidget (Variables|Default|GetEndDialog))
      (Development|SetHiddeninGame (Variables|Default|GetNotification) true false)
      (else
        (Variables|/Game/HUD/DialogWidget.DialogWidget_C|SetLine _dialogwidget (Variables|Default|GetMidDialog))))
    (else
      (Variables|/Game/HUD/DialogWidget.DialogWidget_C|SetLine _dialogwidget (Variables|Default|GetStartDialog))
      (Variables|Default|SetStarted? true))))