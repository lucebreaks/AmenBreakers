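; Quest actor for a timed letter hunt, with five letters tracked on the player character.
; Ready spawns indexed Letter_Blueprint actors at the LetterPos markers, rotated 90 degrees in roll, and DialogFinished unhides them after NPC dialog.
; TimerEvent hides the letters and timer widget and resets the player's Letters array on timeout.
; CheckFinished pauses the timer, started outside these graphs, once every Letters entry is true.
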(event EventTimerEvent
  ;[1 1 1] reset progress on timeout
  (bind _outactors (Actor|GetAllActorsOfClass "/Game/SprayDecals/Letter_Blueprint.Letter_Blueprint_C"))
  (for _array_element _outactors
    (Rendering|SetActorHiddenInGame _array_element true))
  (Widget|SetVisibility (Variables|Default|GetTimerWidget) "Hidden")
  (bind _asbp_player_character (Utilities|Casting|CastToBP_PlayerCharacter (Game|GetPlayerCharacter 0)))
  (for (_ _array_index) (Variables|/Game/Actors/Blueprints/BP_PlayerCharacter.BP_PlayerCharacter_C|GetLetters _asbp_player_character)
    (Utilities|Array|SetArrayElem (Variables|/Game/Actors/Blueprints/BP_PlayerCharacter.BP_PlayerCharacter_C|GetLetters _asbp_player_character) _array_index false)))

(event EventDialogFinished
  ;[1 1 1] After talking to the NPC, make letters visible
  (bind _outactors (Actor|GetAllActorsOfClass "/Game/SprayDecals/Letter_Blueprint.Letter_Blueprint_C"))
  (for _array_element _outactors
    (Rendering|SetActorHiddenInGame _array_element false)))

(event EventReady
  ;[1 1 1] Spawn letters at LetterPos and mark what letter they are
  (for (_array_element _array_index) (Utilities|Array|MakeArray (Variables|Default|GetLetterPos0) (Variables|Default|GetLetterPos1) (Variables|Default|GetLetterPos2) (Variables|Default|GetLetterPos3) (Variables|Default|GetLetterPos4))
    (bind _returnvalue (Game|SpawnActorfromClass "/Game/SprayDecals/Letter_Blueprint.Letter_Blueprint_C" (Math|Transform|MakeTransform (.Location (Math|Transform|BreakTransform (Transformation|GetWorldTransform _array_element))) (Math|Rotator|MakeRotator (+ (.Roll (Math|Rotator|BreakRotator (.Rotation (Math|Transform|BreakTransform (Transformation|GetWorldTransform _array_element))))) 9e+01) (.Pitch (Math|Rotator|BreakRotator (.Rotation (Math|Transform|BreakTransform (Transformation|GetWorldTransform _array_element))))) (.Yaw (Math|Rotator|BreakRotator (.Rotation (Math|Transform|BreakTransform (Transformation|GetWorldTransform _array_element)))))) (.Scale (Math|Transform|BreakTransform (Transformation|GetWorldTransform _array_element)))) "Undefined" 0 0))
    (Variables|/Game/SprayDecals/Letter_Blueprint.Letter_Blueprint_C|SetLetterIndex _returnvalue _array_index)
    (Default|Ready _returnvalue)))

(fn ConstructionScript
  (|CallParentFunction))

(fn CheckFinished
  (bind _asbp_player_character (Utilities|Casting|CastToBP_PlayerCharacter (Game|GetPlayerCharacter 0)))
  (bind _array_element (Utilities|Array|ForEachLoopwithBreak (Variables|/Game/Actors/Blueprints/BP_PlayerCharacter.BP_PlayerCharacter_C|GetLetters _asbp_player_character) :!label _label)
    (:LoopBody
      (bind _output_get (Variables|Default|SetFinished? _array_element))
      (if (not _output_get)
        (goto _label Break)))
    (:Completed
      (if (Variables|Default|GetFinished?)
        (Utilities|Time|PauseTimerbyHandle (Variables|Default|GetTimerHandle))))))